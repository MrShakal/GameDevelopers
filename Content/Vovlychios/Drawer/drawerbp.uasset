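; Interactable drawer that slides open or closed each time its Interactwith event fires.
; A FlipFlop alternates between playing and reversing a timeline, with an open or close sound at the actor's location.
; The timeline lerps Drawer1's relative location between the Close and Open vectors.
; A DoOnce gate, reset through a short delay fired from the timeline update, briefly blocks repeat interaction.
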(event `/Game/Character/InspectInterface.InteractWith`
  (params (PlayerCharacter :type "/Game/Character/BP_PlayerCharacter Object Reference"))
  (cast `/Game/Character/BP_PlayerCharacter` (`GameplayStatics.GetPlayerCharacter` 0))
  (if true
    (`/Engine/EditorBlueprintResources/StandardMacros.DoOnce` false :!label _label
      (:`Completed`
        (`/Engine/EditorBlueprintResources/StandardMacros.FlipFlop`
          (:`A`
            (`GameplayStatics.SpawnSoundAtLocation` "/Game/Audio/open_door.open_door" (`self.K2_GetActorLocation`) (struct) 1.0 1.0 0.0 null null)
            (bind (_direction _open) (`Timeline|Timeline` :!via `PlayFromStart` :!label _label_2)
              (:`Update`
                (`SceneComponent.K2_SetRelativeLocation` (`self.Drawer_1`) (`KismetMathLibrary.VLerp` (`self.Close`) (`self.Open`) _open) false false)
                (`KismetSystemLibrary.Delay` 0.2)
                (goto _label :!via `Reset`))))
          (:`B`
            (`GameplayStatics.SpawnSoundAtLocation` "/Game/Audio/close_door.close_door" (`self.K2_GetActorLocation`) (struct) 1.0 1.0 0.0 null null)
            (goto _label_2 :!via `Reverse`)))))))

(fn `UserConstructionScript`)