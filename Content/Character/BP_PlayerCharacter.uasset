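; BP_PlayerCharacter is the player character, with axis-driven walking, mouse look, a toggleable flashlight and a store of collected keys.
; A FlipFlop switches the SpotLight with on/off sounds, mouse X also sets TurnRate, and BeginPlay adds the HUD widget.
; AddKey and IsKey add to and query the KeyUP collection.
; E fires a debug-drawn camera line trace whose result is not yet used.
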(event `InputAction|Flash On OFF`
  (params (Key :type "Key Structure"))
  (bind _spotlight (`self.SpotLight`))
  (bind _returnvalue (`SceneComponent.K2_GetComponentLocation` _spotlight))
  (:`Pressed`
    (`/Engine/EditorBlueprintResources/StandardMacros.FlipFlop`
      (:`A`
        (`GameplayStatics.PlaySoundAtLocation` "/Game/Flash/Flashlight_On.Flashlight_On" _returnvalue (struct) 1.0 1.0 0.0 null null null null)
        (`SceneComponent.SetVisibility` _spotlight true false))
      (:`B`
        (`GameplayStatics.PlaySoundAtLocation` "/Game/Flash/Flashlight_Off.Flashlight_Off" _returnvalue (struct) 1.0 1.0 0.0 null null null null)
        (`SceneComponent.SetVisibility` _spotlight false false)))))

(event `InputAxis|WalkForward`
  (params (AxisValue :type "Float (single-precision)"))
  ;[1 1 1] Передвижение
  (`self.AddMovementInput` (`KismetMathLibrary.GetForwardVector` (`self.GetControlRotation`)) AxisValue))

(event `Key|E`
  (params (Key :type "Key Structure"))
  (bind _cameraplayer (`self.CameraPlayer`))
  (bind _returnvalue (`SceneComponent.K2_GetComponentLocation` _cameraplayer))
  (:`Pressed`
    (`KismetSystemLibrary.LineTraceSingle` :`Start` _returnvalue :`End` (+ (* (`SceneComponent.GetForwardVector` _cameraplayer) 500.0) _returnvalue) :`TraceChannel` "TraceTypeQuery1" :`bTraceComplex` true :`DrawDebugType` "ForDuration")))

(event `InputAxis|WalkRight`
  (params (AxisValue :type "Float (single-precision)"))
  ;[1 1 1] Передвижение
  (`self.AddMovementInput` (`KismetMathLibrary.GetRightVector` (`self.GetControlRotation`)) AxisValue))

(event `InputAxis|Mouse X`
  (params (AxisValue :type "Float (single-precision)"))
  ;[1 1 1] camera
  (`self.AddControllerYawInput` AxisValue)
  (set `self.turnRate` AxisValue))

(event `InputAxis|Mouse Y`
  (params (AxisValue :type "Float (single-precision)"))
  ;[1 1 1] camera
  (`self.AddControllerPitchInput` AxisValue))

(event `self.ReceiveBeginPlay`
  (bind _returnvalue (`|CreateWidget` "/Game/UI/HUD.HUD_C"))
  (`UserWidget.AddToViewport` _returnvalue 0))

(fn `AddKey`
  (params (Key :type "Integer (by ref)"))
  (`KismetArrayLibrary.Array_AddUnique` (`self.Key UP`) Key))

(fn `IsKey?`
  (params (Key :type "Integer (by ref)"))
  (returns (ReturnValue :type Boolean))
  (return (`KismetArrayLibrary.Array_Contains` (`self.Key UP`) Key)))

(fn `UserConstructionScript`)