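; BP_InspectParent is a base actor for physics objects the player can pick up and inspect, one at a time.
; Interactwith, if the player holds no item, disables character input, takes input itself, attaches to the character's Item component and moves in front of the camera with physics and collision off.
; IA_StopingInspect resets the relative transform, detaches, restores physics and collision, and clears the player's CurrentItem.
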(event `/Game/Character/InspectInterface.InteractWith`
  (params (PlayerCharacter :type "/Game/Character/BP_PlayerCharacter Object Reference"))
  (bind _output_get (set `self.Player Character` PlayerCharacter))
  (`/Game/Character/BP_PlayerCharacter.CurrentItem` _output_get
    (:`then`)
    (:`else`
      (`self.StartInspect`))))

(event `EnhancedInput|/Game/FirstPerson/Input/Actions/IA_StopingInspect`
  (params (ActionValue :type Boolean) (ElapsedSeconds :type "Float (double-precision)") (TriggeredSeconds :type "Float (double-precision)") (InputAction :type "InputAction Object Reference" :default "/Game/FirstPerson/Input/Actions/IA_StopingInspect.IA_StopingInspect"))
  (:`Started`
    (`self.StopInspect`)
    (set `/Game/Character/BP_PlayerCharacter.CurrentItem` null (stale `/Game/Character/InspectInterface.InteractWith` _output_get))))

(fn `StartInspect`
  (bind _returnvalue (`GameplayStatics.GetPlayerController` 0))
  (bind _returnvalue_2 (`GameplayStatics.GetPlayerCameraManager` 0))
  (bind _inspectmesh (`self.InspectMesh`))
  (bind _player_character (`self.Player Character`))
  (`self.DisableInput` _player_character _returnvalue)
  (`self.EnableInput` _returnvalue)
  (`self.K2_AttachToComponent` (`/Game/Character/BP_PlayerCharacter.Item` _player_character) "None" "SnapToTarget" "SnapToTarget" "KeepRelative")
  (`PrimitiveComponent.SetSimulatePhysics` _inspectmesh false)
  (`PrimitiveComponent.SetCollisionEnabled` _inspectmesh "NoCollision")
  (set `/Game/Character/BP_PlayerCharacter.CurrentItem` self (`self.Player Character`))
  (`self.K2_SetActorLocation` (+ (`PlayerCameraManager.GetCameraLocation` _returnvalue_2) (* (`KismetMathLibrary.GetForwardVector` (`PlayerCameraManager.GetCameraRotation` _returnvalue_2)) 200.0))))

(fn `StopInspect`
  (bind _returnvalue (`GameplayStatics.GetPlayerController` 0))
  (bind _inspectmesh (`self.InspectMesh`))
  (`self.DisableInput` _returnvalue)
  (`self.EnableInput` _returnvalue)
  (`self.K2_SetActorRelativeLocation` (0.0 0.0 0.0))
  (`self.K2_SetActorRelativeRotation` (struct))
  (`self.K2_DetachFromActor` "KeepWorld" "KeepWorld" "KeepWorld")
  (`PrimitiveComponent.SetSimulatePhysics` _inspectmesh true)
  (`PrimitiveComponent.SetCollisionEnabled` _inspectmesh "QueryAndPhysics"))

(fn `UserConstructionScript`)