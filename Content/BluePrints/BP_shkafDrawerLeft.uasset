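; BP_shkafDrawerLeft is an interactable left cabinet drawer that opens and closes on player interaction.
; Interactwith alternates through a FlipFlop, playing open or close sounds and running a timeline forward or backward to lerp the drawer's position.
; A DoOnce blocks repeat triggers until a delay after timeline updates resets it.
; IsSelect and NotSelect share a looping MultiGate that toggles the drawer's custom-depth stencil highlight.
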(event `/Game/Character/InspectInterface.InteractWith`
  (params (PlayerCharacter :type "/Game/Character/BP_PlayerCharacter Object Reference") (key :type "Key Structure"))
  (cast `/Game/Character/BP_PlayerCharacter` (`GameplayStatics.GetPlayerCharacter` 0))
  (if true
    (`/Engine/EditorBlueprintResources/StandardMacros.DoOnce` false :!label _label
      (:`Completed`
        (`/Engine/EditorBlueprintResources/StandardMacros.FlipFlop`
          (:`A`
            (`GameplayStatics.SpawnSoundAtLocation` "/Game/Vovlychios/Drawer/Texture/Drawer_Open.Drawer_Open" (`self.K2_GetActorLocation`) (struct) 1.0 1.0 0.0 null null)
            (bind (_direction _open) (`Timeline|Timeline` :!via `PlayFromStart` :!label _label_2)
              (:`Update`
                (`SceneComponent.K2_SetRelativeLocation` (`self.LeftDrawer`) (`KismetMathLibrary.VLerp` (`self.Close`) (`self.Open`) _open) false false)
                (`KismetSystemLibrary.Delay` 1.2)
                (goto _label :!via `Reset`))))
          (:`B`
            (`GameplayStatics.SpawnSoundAtLocation` "/Game/Vovlychios/Drawer/Texture/Drawer_Close.Drawer_Close" (`self.K2_GetActorLocation`) (struct) 1.0 1.0 0.0 null null)
            (goto _label_2 :!via `Reverse`)))))))

(event `/Game/Interaction/BI_selected.IsSelect`
  (bind _leftdrawer (`self.LeftDrawer`))
  (`|MultiGate` false true :!label _label_3
    (:`Out 0`
      (`PrimitiveComponent.SetRenderCustomDepth` _leftdrawer true)
      (`PrimitiveComponent.SetCustomDepthStencilValue` _leftdrawer 2))
    (:`Out 1`
      (`PrimitiveComponent.SetRenderCustomDepth` _leftdrawer false)
      (`PrimitiveComponent.SetCustomDepthStencilValue` _leftdrawer 0))))

(event `/Game/Interaction/BI_selected.NotSelect`
  (goto _label_3))

(fn `IsSelected?`
  (returns (`select?` :type Boolean))
  (return false))

(fn `UserConstructionScript`)