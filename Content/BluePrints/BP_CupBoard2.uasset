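; Interactable cupboard whose right door swings open and closed with sound when the player interacts.
; A FlipFlop plays or reverses a rotation timeline between CloseAngle and OpenAngle, with a delayed DoOnce reset blocking repeated triggers.
; A forced-open branch with a sound and slight door nudge exists, but its constant-true condition leaves it unreachable.
; IsSelect and NotSelect share a looping MultiGate that toggles the door's custom-depth stencil highlight.
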(event `/Game/Character/InspectInterface.InteractWith`
  (params (PlayerCharacter :type "/Game/Character/BP_PlayerCharacter Object Reference") (key :type "Key Structure"))
  (cast `/Game/Character/BP_PlayerCharacter` (`GameplayStatics.GetPlayerCharacter` 0))
  (if true
    (`/Engine/EditorBlueprintResources/StandardMacros.DoOnce` false :!label _label
      (:`Completed`
        (`/Engine/EditorBlueprintResources/StandardMacros.FlipFlop`
          (:`A`
            (`GameplayStatics.SpawnSoundAtLocation` "/Game/Audio/open_door.open_door" (`self.K2_GetActorLocation`) (struct) 1.0 1.0 0.0 null null)
            (bind (_direction _open) (`Timeline|Timeline_0` :!via `PlayFromStart` :!label _label_2)
              (:`Update`
                (`SceneComponent.K2_SetRelativeRotation` (`self.rightdoor`) (`KismetMathLibrary.MakeRotator` 0.0 0.0 (`KismetMathLibrary.Lerp` (`self.close angle`) (`self.open angle`) _open)) false false)
                (`KismetSystemLibrary.Delay` 1.2)
                (goto _label :!via `Reset`))))
          (:`B`
            (`GameplayStatics.SpawnSoundAtLocation` "/Game/Audio/close_door.close_door" (`self.K2_GetActorLocation`) (struct) 1.0 1.0 0.0 null null)
            (goto _label_2 :!via `Reverse`)))))
    (else
      (`/Engine/EditorBlueprintResources/StandardMacros.DoOnce` false :!label _label_3
        (:`Completed`
          (`GameplayStatics.PlaySound2D` "/Game/Audio/pytaeshsya-otkryt-siloy-51.pytaeshsya-otkryt-siloy-51" 1.0 1.0 0.0 null null)
          (if true
            (bind (_direction_2 _door) (`Timeline|Timeline` :!via `PlayFromStart`)
              (:`Update`
                (`SceneComponent.K2_SetRelativeRotation` (`self.rightdoor`) (`KismetMathLibrary.MakeRotator` 0.0 0.0 (`KismetMathLibrary.Lerp` 0.0 -1.0 _door)) false false)
                (`KismetSystemLibrary.Delay` 1.5)
                (goto _label_3 :!via `Reset`)))))))))

(event `/Game/Interaction/BI_selected.IsSelect`
  (bind _rightdoor (`self.rightdoor`))
  (`|MultiGate` false true :!label _label_4
    (:`Out 0`
      (`PrimitiveComponent.SetRenderCustomDepth` _rightdoor true)
      (`PrimitiveComponent.SetCustomDepthStencilValue` _rightdoor 2))
    (:`Out 1`
      (`PrimitiveComponent.SetRenderCustomDepth` _rightdoor false)
      (`PrimitiveComponent.SetCustomDepthStencilValue` _rightdoor 0))))

(event `/Game/Interaction/BI_selected.NotSelect`
  (goto _label_4))

(fn `IsSelected?`
  (returns (`select?` :type Boolean))
  (return false))

(fn `UserConstructionScript`)