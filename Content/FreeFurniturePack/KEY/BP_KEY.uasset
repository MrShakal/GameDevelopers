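; BP_KEY is a key pickup that the player can highlight and collect.
; Interacting sets HasKey on BP_PlayerCharacter, plays a sound at the key's location and destroys the actor.
; IsSelect and NotSelect share a looping MultiGate that alternately turns Key9's custom depth stencil highlight on and off, so the state follows call order rather than which event fired.
; IsSelected always returns false.
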(event `/Game/Character/InspectInterface.InteractWith`
  (params (PlayerCharacter :type "/Game/Character/BP_PlayerCharacter Object Reference"))
  (bind _asbp_player_character (cast `/Game/Character/BP_PlayerCharacter` (`GameplayStatics.GetPlayerCharacter` 0)))
  (set `/Game/Character/BP_PlayerCharacter.Has Key?` true _asbp_player_character)
  (`GameplayStatics.PlaySoundAtLocation` "/Game/Flash/zvon-kljuchej_1___online-audio-converter_com___1_.zvon-kljuchej_1___online-audio-converter_com___1_" (`self.K2_GetActorLocation`) (struct) 1.0 1.0 0.0 null null null null)
  (`self.K2_DestroyActor`))

(event `/Game/Interaction/BI_selected.IsSelect`
  (bind _key9 (`self.Key9`))
  (`|MultiGate` false true :!label _label
    (:`Out 0`
      (`PrimitiveComponent.SetRenderCustomDepth` _key9 true)
      (`PrimitiveComponent.SetCustomDepthStencilValue` _key9 2))
    (:`Out 1`
      (`PrimitiveComponent.SetRenderCustomDepth` _key9 false)
      (`PrimitiveComponent.SetCustomDepthStencilValue` _key9 0))))

(event `/Game/Interaction/BI_selected.NotSelect`
  (goto _label))

(fn `IsSelected?`
  (returns (`select?` :type Boolean))
  (return false))

(fn `UserConstructionScript`)