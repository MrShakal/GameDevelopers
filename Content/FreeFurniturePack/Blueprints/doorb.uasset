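; Draggable door actor that the player swings by holding the DragDoor input and turning.
; On press, a 500-unit camera line trace checks for any doorb actor, not specifically this instance.
; While held, Tick adds the player's TurnRate times Sensitivity to the door's yaw.
; When world yaw leaves the ±OpenAngle range, relative yaw snaps to one degree inside the limit.
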(event `self.ReceiveTick`
  (params (DeltaSeconds :type "Float (single-precision)"))
  (bind _open_angle (`self.Open Angle`))
  (bind _door (`self.Door`))
  (bind (_returnvalue_roll _returnvalue_pitch _returnvalue_yaw) (`KismetMathLibrary.BreakRotator` (`SceneComponent.K2_GetComponentRotation` (`self.Door`))))
  (if (`self.IsHoldingLBM`)
    (if (`self.IsLookingADoor`)
      (if (not (== _returnvalue_yaw (`KismetMathLibrary.ClampAngle` _returnvalue_yaw _open_angle (* _open_angle -1.0))))
        (`SceneComponent.K2_AddLocalRotation` _door (`KismetMathLibrary.MakeRotator` 0.0 0.0 (* (`/Game/Character/BP_PlayerCharacter.turnRate` (stale `InputAction|DragDoor` _asbp_player_character)) (`self.Sensitivity`))) false false)
        (elif (>= _returnvalue_yaw _open_angle)
          (`SceneComponent.K2_SetRelativeRotation` _door (`KismetMathLibrary.MakeRotator` 0.0 0.0 (- _open_angle 1.0)) false false)
          (else
            (`SceneComponent.K2_SetRelativeRotation` _door (`KismetMathLibrary.MakeRotator` 0.0 0.0 (+ (* _open_angle -1.0) 1.0)) false false)))))))

(event `self.ReceiveBeginPlay`
  ;[1 1 1] вкл кнопки мыши лкм
  (`self.EnableInput` (`GameplayStatics.GetPlayerController` 0)))

(event `InputAction|DragDoor`
  (params (Key :type "Key Structure"))
  ;[1 1 1] смотрим на дверь
  (:`Pressed`
    (set `self.IsHoldingLBM` true)
    (bind _asbp_player_character (cast `/Game/Character/BP_PlayerCharacter` (`GameplayStatics.GetPlayerCharacter` 0)))
    (bind _cameraplayer (`/Game/Character/BP_PlayerCharacter.CameraPlayer` _asbp_player_character))
    (bind _returnvalue (`SceneComponent.K2_GetComponentLocation` _cameraplayer))
    (bind (_outhit _returnvalue_2) (`KismetSystemLibrary.LineTraceSingleForObjects` :`Start` _returnvalue :`End` (+ _returnvalue (* (`SceneComponent.GetForwardVector` _cameraplayer) 500.0)) :`ObjectTypes` (`|MakeArray` "ObjectTypeQuery2" :!type "EObjectTypeQuery Enum") :`bIgnoreSelf` false))
    (if _returnvalue_2
      (cast `/Game/FreeFurniturePack/Blueprints/doorb` (`.HitActor` (`GameplayStatics.BreakHitResult` _outhit)))
      (set `self.IsLookingADoor` true)
      (else
        (set `self.IsLookingADoor` false))))
  (:`Released`
    (set `self.IsHoldingLBM` false)))

(fn `UserConstructionScript`)